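; A guard AI Blueprint that patrols, chases the player on sight and resets the player on melee contact.
; Each tick, a view-cone, range and visibility line trace check records the sighting time and raises local and level alarms.
; It pursues the player's current position until a no-sight timeout expires, then changes alarm status and resumes patrol.
; A player reset clears the sighting and patrol interruption.
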(event `self.ReceiveBeginPlay`
  (`parent.ReceiveBeginPlay`))

(event `self.ReceiveTick`
  (params (DeltaSeconds :type "Float (single-precision)"))
  (`parent.ReceiveTick` DeltaSeconds)
  (`|ExecutionSequence`
    (:`then_0`
      (bind _visible (`self.PlayerVisible?`))
      (if _visible
        (set `self.lastSeenTime` (`GameplayStatics.GetTimeSeconds`))
        (set `self.LocalAlarmStatus` "NewEnumerator0")
        (`/Game/CalShit/Security/LevelManager_BP.Update Alarm Status` (`self.LevelManagerRef`) "NewEnumerator0")))
    (:`then_1`
      (if (< (- (`GameplayStatics.GetTimeSeconds`) (`self.lastSeenTime`)) (`self.noSightTrackTime`))
        (set `self.PatrolInterupt` true)
        (`|AIMoveTo` self (`self.K2_GetActorLocation` (`self.PlayerRef`)) null)
        (elif (`self.PatrolInterupt`)
          (set `self.PatrolInterupt` false)
          (set `self.LocalAlarmStatus` "NewEnumerator3")
          (`self.Cycle Patrol Behavior`))))))

(event `self.MeleeCollision.OnComponentBeginOverlap`
  (params (OverlappedComponent :type "PrimitiveComponent Object Reference") (OtherActor :type "Actor Object Reference") (OtherComp :type "PrimitiveComponent Object Reference") (OtherBodyIndex :type Integer) (bFromSweep :type Boolean) (SweepResult :type "HitResult Structure (by ref)"))
  (cast `/Game/TylerShit/Player_BP` OtherActor)
  (cast `CapsuleComponent` OtherComp)
  (`/Game/CalShit/Security/LevelManager_BP.Player Reset` (`self.LevelManagerRef`)))

(fn `On Player Reset Extras`
  (`parent.On Player Reset Extras`)
  (set `self.lastSeenTime` -100.0)
  (set `self.PatrolInterupt` false))

(fn `PlayerVisible?`
  (returns (Visible :type Boolean))
  (`|ExecutionSequence`
    (:`then_0`
      (if (< (`KismetMathLibrary.DegCos` (`self.viewHalfAngle`)) (`KismetMathLibrary.Vector_CosineAngle2D` (- (`self.K2_GetActorLocation` (`self.PlayerRef`)) (`self.K2_GetActorLocation`)) (`self.GetActorForwardVector`)))
        (if (< (`KismetMathLibrary.VSizeSquared` (- (`self.K2_GetActorLocation` (`self.PlayerRef`)) (`self.K2_GetActorLocation`))) (`KismetMathLibrary.Square` (`self.viewRange`)))
          (bind (_outhit _returnvalue) (`KismetSystemLibrary.LineTraceSingle` :`Start` (`self.K2_GetActorLocation`) :`End` (`self.K2_GetActorLocation` (`self.PlayerRef`)) :`TraceChannel` "TraceTypeQuery1" :`DrawDebugType` "ForDuration"))
          (return (not _returnvalue)))))
    (:`then_1`
      (return false))))

(fn `UserConstructionScript`
  (`parent.UserConstructionScript`))