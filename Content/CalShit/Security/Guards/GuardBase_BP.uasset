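; Base guard Blueprint that registers with LevelManager_BP and loops through a list of Move and Wait patrol behaviors.
; Moves use SimpleMoveToLocation on the AI controller; Tick advances on arrival within tolerance or after Value.X seconds, printing remaining distance while moving.
; The construction script passes each entry to AddPatrolBehavior, which creates arrow markers for Move points but also re-appends to the array being iterated.
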(event `self.ReceiveBeginPlay`
  (bind _returnvalue (`GameplayStatics.GetActorOfClass` "/Game/CalShit/Security/LevelManager_BP.LevelManager_BP_C"))
  (bind _output_get (set `self.LevelManagerRef` _returnvalue))
  (`KismetArrayLibrary.Array_Add` (`/Game/CalShit/Security/LevelManager_BP.GuardRefs` _output_get) self)
  (set `self.CurrentPatrolState` (`self.InitialPatrolState`))
  (bind _asaicontroller (cast `AIController` (`self.GetController`)))
  (set `self.SelfControllerRef` _asaicontroller)
  (`self.Cycle Patrol Behavior`))

(event `self.ReceiveTick`
  (params (DeltaSeconds :type "Float (single-precision)"))
  (`self.Check For Patrol Completion`))

(fn `Add Patrol Behavior`
  (params (`New Patrol Behavior` :type "/Game/CalShit/Security/Guards/PatrolBehavior_S Structure"))
  (`KismetArrayLibrary.Array_Add` (`self.PatrolBehavior`) `New Patrol Behavior`)
  (`self.Add Patrol Behavior Visulizer` `New Patrol Behavior`))

(fn `Add Patrol Behavior Visulizer`
  (params (Behavior :type "/Game/CalShit/Security/Guards/PatrolBehavior_S Structure"))
  (bind (_type _value) (break `/Game/CalShit/Security/Guards/PatrolBehavior_S` Behavior))
  (bind _behavior_arrow_length (`self.Behavior Arrow Length`))
  (switch `/Game/CalShit/Security/Guards/PatrolBehaviorTypes_E` _type
    (:`NewEnumerator0`
      (bind _returnvalue (`AddComponent|NODE_AddArrowComponent-0` :`RelativeTransform` (`KismetMathLibrary.MakeTransform` (+ (`KismetMathLibrary.InverseTransformLocation` (`SceneComponent.K2_GetComponentToWorld` (`self.CapsuleComponent`)) _value) (`KismetMathLibrary.MakeVector` 0.0 0.0 (* _behavior_arrow_length (`self.Behavior Arrow Size`)))) (struct :`Pitch` -90.0))))
      (set `ArrowComponent.ArrowLength` _behavior_arrow_length _returnvalue)
      (set `ArrowComponent.ArrowSize` (`self.Behavior Arrow Size`) _returnvalue)
      (`KismetArrayLibrary.Array_Add` (`self.Behavior Visualizers`) _returnvalue))))

(fn `Check For Patrol Completion`
  (bind (_type _value) (break `/Game/CalShit/Security/Guards/PatrolBehavior_S` (`self.CurrentPatrolBehavior`)))
  (bind _returnvalue (`KismetMathLibrary.VSize` (- (`self.K2_GetActorLocation` self) _value)))
  (switch `/Game/CalShit/Security/Guards/PatrolBehaviorTypes_E` _type
    (:`NewEnumerator0`
      (if (< _returnvalue (`self.PatrolPositionTolerance`))
        (`self.Cycle Patrol Behavior`)
        (else
          (`KismetSystemLibrary.PrintString` (`KismetStringLibrary.Conv_DoubleToString` _returnvalue)))))
    (:`NewEnumerator2`
      (if (>= (`GameplayStatics.GetTimeSeconds`) (+ (`self.PatrolBehaviorStartTime`) (.x _value)))
        (`self.Cycle Patrol Behavior`)))))

(fn `Cycle Patrol Behavior`
  (`/Engine/EditorBlueprintResources/StandardMacros.IncrementInt` (`self.CurrentPatrolState`)
    (:`  `
      (set `self.CurrentPatrolState` (mod (`self.CurrentPatrolState`) (`KismetArrayLibrary.Array_Length` (`self.PatrolBehavior`))))
      (bind _output_get (set `self.CurrentPatrolBehavior` (`|GetArrayItem` (`self.PatrolBehavior`) (`self.CurrentPatrolState`))))
      (`self.Execute Patrol Behavior` _output_get))))

(fn `Execute Patrol Behavior`
  (params (`Patrol Behavior` :type "/Game/CalShit/Security/Guards/PatrolBehavior_S Structure"))
  (bind (_type _value) (break `/Game/CalShit/Security/Guards/PatrolBehavior_S` `Patrol Behavior`))
  (set `self.PatrolBehaviorStartTime` (`GameplayStatics.GetTimeSeconds`))
  (switch `/Game/CalShit/Security/Guards/PatrolBehaviorTypes_E` _type
    (:`NewEnumerator0`
      (`AIBlueprintHelperLibrary.SimpleMoveToLocation` (`self.SelfControllerRef`) _value))))

(fn `Remove Last Behavior`
  (bind _patrolbehavior (`self.PatrolBehavior`))
  (bind _behavior_visualizers (`self.Behavior Visualizers`))
  (bind _behavior_visualizers_2 (`self.Behavior Visualizers`))
  (`|ExecutionSequence`
    (:`then_0`
      (`ActorComponent.K2_DestroyComponent` (`|GetArrayItem` _behavior_visualizers (`KismetArrayLibrary.Array_LastIndex` _behavior_visualizers))))
    (:`then_1`
      (`KismetArrayLibrary.Array_Remove` _patrolbehavior (`KismetArrayLibrary.Array_LastIndex` _patrolbehavior))
      (`KismetArrayLibrary.Array_Remove` _behavior_visualizers_2 (`KismetArrayLibrary.Array_LastIndex` _behavior_visualizers_2)))))

(fn `Update Patrol Behavior Visulizer`)

(fn `UserConstructionScript`
  (for _array_element (`self.PatrolBehavior`)
    (`self.Add Patrol Behavior` _array_element)))