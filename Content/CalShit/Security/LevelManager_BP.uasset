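; Level manager for a security/stealth level that handles player resets and the level-wide alarm state.
; On BeginPlay it caches the player controller, the Player_BP pawn and the player's starting transform.
; PlayerReset returns the player and control rotation to that start and notifies each referenced guard.
; UpdateAlarmStatus stores the global alarm status and pushes it to all referenced guards and security devices.
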(event `self.ReceiveBeginPlay`
  (`|ExecutionSequence`
    (:`then_0`
      (set `self.PlayerControllerRef` (`GameplayStatics.GetPlayerController` 0))
      (bind _asplayer_bp (cast `/Game/TylerShit/Player_BP` (`GameplayStatics.GetPlayerPawn` 0)))
      (bind _output_get (set `self.PlayerRef` _asplayer_bp))
      (set `self.PlayerInitLoc` (`self.K2_GetActorLocation` _output_get))
      (set `self.PlayerInitRot` (`self.K2_GetActorRotation` _output_get)))))

(fn `Player Reset`
  (`self.K2_SetActorLocationAndRotation` (`self.PlayerRef`) (`self.PlayerInitLoc`) (`self.PlayerInitRot`) false false)
  (`Controller.SetControlRotation` (`self.PlayerControllerRef`) (`self.PlayerInitRot`))
  (for _array_element (`self.GuardRefs`)
    (`/Game/CalShit/Security/Guards/GuardBase_BP.On Player Reset` _array_element)))

(fn `Update Alarm Status`
  (params (`New Alarm Status` :type "/Game/CalShit/Security/AlarmStatus_E Enum" :default "NewEnumerator0"))
  (bind _output_get (set `self.GlobalAlarmStatus` `New Alarm Status`))
  (`|ExecutionSequence`
    (:`then_0`
      (for _array_element (`self.GuardRefs`)
        (set `/Game/CalShit/Security/Guards/GuardBase_BP.GlobalAlarmStatus` _output_get _array_element)))
    (:`then_1`
      (for _array_element_2 (`self.SecDeviceRefs`)
        (set `/Game/CalShit/Security/Devices/SecurityDeviceBase_BP.GlobalAlarmStatus` _output_get _array_element_2)))))

(fn `UserConstructionScript`)