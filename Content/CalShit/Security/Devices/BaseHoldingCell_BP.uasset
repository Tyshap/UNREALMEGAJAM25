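; Base holding cell security device that tracks whether the player leaves the cell in a way that would trigger the guards.
; SafeZone overlaps toggle an InSafeZone flag for the player.
; When the player's overlap with DangerZone ends outside the safe zone, it sets LocalAlarmStatus to a fixed enum state.
; Nothing in these graphs reads that status or alerts guards directly.
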(event `self.SafeZone.OnComponentBeginOverlap`
  (params (OverlappedComponent :type "PrimitiveComponent Object Reference") (OtherActor :type "Actor Object Reference") (OtherComp :type "PrimitiveComponent Object Reference") (OtherBodyIndex :type Integer) (bFromSweep :type Boolean) (SweepResult :type "HitResult Structure (by ref)"))
  ; Determines if player is not going to trigger the guards
  (cast `/Game/TylerShit/Player_BP` OtherActor)
  (set `self.InSafeZone?` true))

(event `self.SafeZone.OnComponentEndOverlap`
  (params (OverlappedComponent :type "PrimitiveComponent Object Reference") (OtherActor :type "Actor Object Reference") (OtherComp :type "PrimitiveComponent Object Reference") (OtherBodyIndex :type Integer))
  ; Determines if player is not going to trigger the guards
  (cast `/Game/TylerShit/Player_BP` OtherActor)
  (set `self.InSafeZone?` false))

(event `self.DangerZone.OnComponentEndOverlap`
  (params (OverlappedComponent :type "PrimitiveComponent Object Reference") (OtherActor :type "Actor Object Reference") (OtherComp :type "PrimitiveComponent Object Reference") (OtherBodyIndex :type Integer))
  ; Called when Player leaves cell
  (cast `/Game/TylerShit/Player_BP` OtherActor)
  (if (not (`self.InSafeZone?`))
    (set `self.LocalAlarmStatus` "NewEnumerator0")))

(fn `UserConstructionScript`
  (`parent.UserConstructionScript`))