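; Generated-mesh actor that procedurally builds a randomized circular maze from concentric wall rings.
; On rebuild it revolves a profile per ring, boolean-subtracts box doorways, then appends radial divider walls.
; Door and divider positions are random points snapped to rings or corridors, retried against optional same-ring and linear spacing rules; failed holes are dropped, dividers kept.
; SaveGeometry exports rings, hole cutters and dividers as separate static mesh assets.
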(event `self.OnRebuildGeneratedMesh`
  (params (TargetMesh :type "DynamicMesh Object Reference"))
  (bind _wallthickness (`self.WallThickness`))
  (bind _height (`self.Height`))
  (set `self.ViewMesh` TargetMesh)
  (bind _returnvalue (`GeometryScriptLibrary_SceneUtilityFunctions.CreateDynamicMeshPool`))
  (set `self.MeshPool` _returnvalue)
  (`|ExecutionSequence`
    (:`then_0`
      (`|ExecutionSequence`
        (:`then_0`
          (`|ExecutionSequence`
            (:`then_0`
              (for _index (range (`self.LayerCount`))
                (set `self.CurrentRing` _index)
                (bind _returnvalue_2 (`DynamicMeshPool.RequestMesh` (`self.MeshPool`)))
                (bind _output_get (set `self.RingPoolMesh` _returnvalue_2))
                (`KismetArrayLibrary.Array_Add` (`self.RingPoolMeshes`) _output_get)
                (`GeometryScriptLibrary_MeshPrimitiveFunctions.AppendRevolvePolygon` (`self.RingPoolMesh`) (struct) (struct) (`|MakeArray` (0.0 0.0) (`KismetMathLibrary.MakeVector2D` _wallthickness) (`KismetMathLibrary.MakeVector2D` _wallthickness _height) (`KismetMathLibrary.MakeVector2D` 0.0 _height) :!type "Vector2D Structure") (make `GeometryScriptRevolveOptions` 360.0) (+ (* (`self.CurrentRing`) (`self.SectionWidth`)) (`self.InnerRadius`)) 128 null)
                (`|ExecutionSequence`
                  (:`then_0`
                    (bind _returnvalue_3 (`GeometryScriptLibrary_MeshNormalsFunctions.RecomputeNormals` (`self.RingPoolMesh`) (make `GeometryScriptCalculateNormalsOptions` true true) false null))
                    (`GeometryScriptLibrary_MeshUVFunctions.RecomputeMeshUVs` _returnvalue_3 0 (make `GeometryScriptRecomputeUVsOptions` "SpectralConformal" "PolyGroups") (struct) null))
                  (:`then_1`
                    (`GeometryScriptLibrary_MeshBasicEditFunctions.AppendMesh` (`self.ViewMesh`) (`self.RingPoolMesh`) (struct) false (struct :`CombineMode` "EnableAllMatching") null)))))))
        (:`then_1`
          (`|ExecutionSequence`
            (:`then_0`
              (bind _returnvalue_4 (`DynamicMeshPool.RequestMesh` (`self.MeshPool`)))
              (set `self.HolesPoolMesh` _returnvalue_4)
              (bind _holetransforms (`self.Get Hole Transforms`))
              (for _array_element _holetransforms
                (`GeometryScriptLibrary_MeshPrimitiveFunctions.AppendBox` (`self.HolesPoolMesh`) (struct) _array_element (+ (`self.WallThickness`) (`self.HoleThicknessBuffer`)) (`self.CorridorWidth`) (- (`self.Height`) (* (`self.HoleHieghtOffset`) 2.0)) 0 0 0 "Base" null)))
            (:`then_1`
              (`GeometryScriptLibrary_MeshBooleanFunctions.ApplyMeshBoolean` (`self.ViewMesh`) (struct) (`self.HolesPoolMesh`) (struct) "Subtract" (struct) null))))
        (:`then_2`
          (`|ExecutionSequence`
            (:`then_0`
              (bind _returnvalue_5 (`DynamicMeshPool.RequestMesh` (`self.MeshPool`)))
              (set `self.DividerPoolMesh` _returnvalue_5)
              (bind _walltransforms (`self.Get Wall Transforms`))
              (for _array_element_2 _walltransforms
                (`GeometryScriptLibrary_MeshPrimitiveFunctions.AppendBox` (`self.DividerPoolMesh`) (struct) _array_element_2 (+ (`self.CorridorWidth`) (`self.DividerWallClipDistance`)) (`self.WallThickness`) (`self.Height`) 0 0 0 "Base" null)))
            (:`then_1`
              (bind _returnvalue_6 (`GeometryScriptLibrary_MeshNormalsFunctions.RecomputeNormals` (`self.DividerPoolMesh`) (struct) false null))
              (`GeometryScriptLibrary_MeshUVFunctions.RecomputeMeshUVs` _returnvalue_6 0 (struct) (struct) null))
            (:`then_2`
              (`GeometryScriptLibrary_MeshBasicEditFunctions.AppendMesh` (`self.ViewMesh`) (`self.DividerPoolMesh`) (struct) false (struct :`CombineMode` "EnableAllMatching") null))))
        (:`then_3`
          (if (`self.SaveGeometry?`)
            (`|ExecutionSequence`
              (:`then_0`
                (`GeometryScriptLibrary_CreateNewAssetFunctions.CreateNewStaticMeshAssetFromMesh` (`self.DividerPoolMesh`) "/Game/CalShit/Geometry/DividerWallMesh" (struct) null))
              (:`then_1`
                (`GeometryScriptLibrary_CreateNewAssetFunctions.CreateNewStaticMeshAssetFromMesh` (`self.HolesPoolMesh`) "/Game/CalShit/Geometry/HolesMesh" (struct) null))
              (:`then_2`
                (for (_array_element_3 _array_index) (`self.RingPoolMeshes`)
                  (`GeometryScriptLibrary_CreateNewAssetFunctions.CreateNewStaticMeshAssetFromMesh` _array_element_3 (`KismetStringLibrary.Concat_StrStr` "/Game/CalShit/Geometry/RingMesh_" (`KismetStringLibrary.Conv_IntToString` _array_index)) (struct) null))))))))
    (:`then_1`
      (`self.ReleaseAllComputeMeshes`))))

(fn `Get Hole Transforms`
  (returns (HoleTransforms :type "Array of Transform Structure"))
  (locals (MyHoleLocations :type "Array of Vector2D Structure") (MyCurrentLoc :type "Vector2D Structure") (`MyStopTrying?` :type Boolean) (MyLocationAttemptCount :type Integer) (`MyWasValidLocation?` :type Boolean) (MyHoleRingNums :type "Array of Integer") (MyCurrentRing :type Integer) (MyHoleTransforms :type "Array of Transform Structure"))
  (bind _returnvalue (`KismetMathLibrary.VSize2D` (`local.MyCurrentLoc`)))
  (`|ExecutionSequence`
    (:`then_0`
      (for _ (range (`self.HoleCount`))
        (set `local.MyLocationAttemptCount` 0)
        (set `local.MyStopTrying?` false)
        (set `local.MyWasValidLocation?` true)
        (while (not (`local.MyStopTrying?`))
          (`/Engine/EditorBlueprintResources/StandardMacros.IncrementInt` (`local.MyLocationAttemptCount`)
            (:`  `
              (set `local.MyStopTrying?` true)
              (bind _output_get (set `local.MyCurrentLoc` (`KismetMathLibrary.MakeVector2D` (`KismetMathLibrary.RandomFloat`) (`KismetMathLibrary.RandomFloat`))))
              (bind _output_get_2 (set `local.MyCurrentLoc` (* (- _output_get (0.5 0.5)) (2.0 2.0) (`self.TotalRadius`))))
              (bind (_outdir _outlength) (`KismetMathLibrary.ToDirectionAndLength2D` _output_get_2))
              (bind _returnvalue_2 (`KismetMathLibrary.Round` (* (/ (- _outlength (`self.InnerRadius`)) (- (`self.TotalRadius`) (`self.InnerRadius`))) (`self.LayerCount`))))
              (set `local.MyCurrentRing` _returnvalue_2)
              (set `local.MyCurrentLoc` (* _outdir (+ (* _returnvalue_2 (`self.SectionWidth`)) (`self.InnerRadius`) (0.0 0.0) (/ (`self.WallThickness`) 2.0))))
              (`|ExecutionSequence`
                (:`then_0`
                  (`|ExecutionSequence`
                    (:`then_0`
                      (if (`KismetMathLibrary.BooleanNAND` (< _returnvalue (`self.TotalRadius`)) (> _returnvalue (`self.InnerRadius`)))
                        (set `local.MyStopTrying?` false)))
                    (:`then_1`
                      (if (`self.EnforceHoleSeperation?`)
                        (`|ExecutionSequence`
                          (:`then_0`
                            (if (`self.RingHoleSeperation?`)
                              (for (_array_element _array_index) (`local.MyHoleLocations`)
                                (if (== (`|GetArrayItem` (`local.MyHoleRingNums`) _array_index) (`local.MyCurrentRing`))
                                  (if (< (`KismetMathLibrary.DistanceSquared2D` _array_element (`local.MyCurrentLoc`)) (`KismetMathLibrary.Square` (`self.RingHoleSeperationDistance`)))
                                    (set `local.MyStopTrying?` false))))))
                          (:`then_1`
                            (if (`self.LinearHoleSeperation?`)
                              (for _array_element_2 (`local.MyHoleLocations`)
                                (if (< (`KismetMathLibrary.DistanceSquared2D` _array_element_2 (`local.MyCurrentLoc`)) (`KismetMathLibrary.Square` (`self.LinearHoleSeperationDistance`)))
                                  (set `local.MyStopTrying?` false))))))))))
                (:`then_1`
                  (if (> (`local.MyLocationAttemptCount`) 100)
                    (set `local.MyStopTrying?` true)
                    (set `local.MyWasValidLocation?` false)))))))
        (if (`local.MyWasValidLocation?`)
          (`KismetArrayLibrary.Array_Add` (`local.MyHoleLocations`) (`local.MyCurrentLoc`))
          (`KismetArrayLibrary.Array_Add` (`local.MyHoleRingNums`) (`local.MyCurrentRing`)))))
    (:`then_1`
      (for _array_element_3 (`local.MyHoleLocations`)
        (bind (_x _y) (`KismetMathLibrary.BreakVector2D` _array_element_3))
        (bind _returnvalue_3 (`KismetMathLibrary.MakeVector` _x _y (`self.HoleHieghtOffset`)))
        (`KismetArrayLibrary.Array_Add` (`local.MyHoleTransforms`) (`KismetMathLibrary.MakeTransform` _returnvalue_3 (`KismetMathLibrary.MakeRotFromXZ` _returnvalue_3 (0.0 0.0 1.0)))))
      (return (`local.MyHoleTransforms`)))))

(fn `Get Wall Transforms`
  (returns (WallTransforms :type "Array of Transform Structure"))
  (locals (MyWallLocations :type "Array of Vector2D Structure") (MyCurrentLoc :type "Vector2D Structure") (`MyStopTrying?` :type Boolean) (MyLocationAttemptCount :type Integer) (`MyWasValidLocation?` :type Boolean) (MyWallRingNums :type "Array of Integer") (MyCurrentRing :type Integer) (MyWallTransforms :type "Array of Transform Structure"))
  (bind _returnvalue (`KismetMathLibrary.VSize2D` (`local.MyCurrentLoc`)))
  (`|ExecutionSequence`
    (:`then_0`
      (for _ (range (`self.DividerWallCount`))
        (set `local.MyLocationAttemptCount` 0)
        (set `local.MyStopTrying?` false)
        (while (not (`local.MyStopTrying?`))
          (`/Engine/EditorBlueprintResources/StandardMacros.IncrementInt` (`local.MyLocationAttemptCount`)
            (:`  `
              (set `local.MyStopTrying?` true)
              (bind _output_get (set `local.MyCurrentLoc` (`KismetMathLibrary.MakeVector2D` (`KismetMathLibrary.RandomFloat`) (`KismetMathLibrary.RandomFloat`))))
              (bind _output_get_2 (set `local.MyCurrentLoc` (* (- _output_get (0.5 0.5)) (2.0 2.0) (`self.TotalRadius`))))
              (bind (_outdir _outlength) (`KismetMathLibrary.ToDirectionAndLength2D` _output_get_2))
              (bind _returnvalue_2 (`KismetMathLibrary.Round` (* (/ (- _outlength (`self.InnerRadius`)) (- (`self.TotalRadius`) (`self.InnerRadius`))) (`self.LayerCount`))))
              (set `local.MyCurrentRing` _returnvalue_2)
              (set `local.MyCurrentLoc` (* _outdir (+ (* _returnvalue_2 (`self.SectionWidth`)) (`self.InnerRadius`) (/ (`self.CorridorWidth`) 2.0) (`self.WallThickness`))))
              (`|ExecutionSequence`
                (:`then_0`
                  (`|ExecutionSequence`
                    (:`then_0`
                      (if (`KismetMathLibrary.BooleanNAND` (< _returnvalue (- (`self.TotalRadius`) (`self.SectionWidth`))) (> _returnvalue (`self.InnerRadius`)))
                        (set `local.MyStopTrying?` false)))
                    (:`then_1`
                      (if (`self.EnforceDividerWallSeperation?`)
                        (`|ExecutionSequence`
                          (:`then_0`
                            (if (`self.RingBasedSeperation?`)
                              (for (_array_element _array_index) (`local.MyWallLocations`)
                                (if (== (`|GetArrayItem` (`local.MyWallRingNums`) _array_index) (`local.MyCurrentRing`))
                                  (if (< (`KismetMathLibrary.DistanceSquared2D` _array_element (`local.MyCurrentLoc`)) (`KismetMathLibrary.Square` (`self.RingSeperationDistance`)))
                                    (set `local.MyStopTrying?` false))))))
                          (:`then_1`
                            (if (`self.LinearSeperation?`)
                              (for _array_element_2 (`local.MyWallLocations`)
                                (if (< (`KismetMathLibrary.DistanceSquared2D` _array_element_2 (`local.MyCurrentLoc`)) (`KismetMathLibrary.Square` (`self.LinearSeperationDistance`)))
                                  (set `local.MyStopTrying?` false))))))))))
                (:`then_1`
                  (if (> (`local.MyLocationAttemptCount`) 100)
                    (set `local.MyStopTrying?` true)
                    (set `local.MyWasValidLocation?` false)))))))
        (`KismetArrayLibrary.Array_Add` (`local.MyWallLocations`) (`local.MyCurrentLoc`))
        (`KismetArrayLibrary.Array_Add` (`local.MyWallRingNums`) (`local.MyCurrentRing`))))
    (:`then_1`
      (for _array_element_3 (`local.MyWallLocations`)
        (bind (_x _y) (`KismetMathLibrary.BreakVector2D` _array_element_3))
        (bind _returnvalue_3 (`KismetMathLibrary.MakeVector` _x _y))
        (`KismetArrayLibrary.Array_Add` (`local.MyWallTransforms`) (`KismetMathLibrary.MakeTransform` _returnvalue_3 (`KismetMathLibrary.MakeRotFromXZ` _returnvalue_3 (0.0 0.0 1.0)))))
      (return (`local.MyWallTransforms`)))))

(fn `UserConstructionScript`
  (set `self.SectionWidth` (+ (`self.CorridorWidth`) (`self.WallThickness`)))
  (set `self.TotalRadius` (+ (* (`self.LayerCount`) (`self.SectionWidth`)) (`self.InnerRadius`))))