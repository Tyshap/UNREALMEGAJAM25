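; Generated dynamic mesh actor that scatters radial divider walls across concentric ring layers around an open center, as a level generation tool.
; On rebuild it rejection-samples random points within the annulus, optionally enforcing minimum separation, with limited retries per wall.
; Each point snaps to a ring layer and becomes an outward-facing box spanning the layer width.
; Boxes accumulate in a pooled mesh, which gets recomputed normals before being appended to the target mesh.
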(event `self.OnRebuildGeneratedMesh`
  (params (TargetMesh :type "DynamicMesh Object Reference"))
  (bind (_x _y) (`KismetMathLibrary.BreakVector2D` (`self.CurrentWallLocationClean`)))
  (set `self.ViewMesh` TargetMesh)
  (bind _returnvalue (`GeometryScriptLibrary_SceneUtilityFunctions.CreateDynamicMeshPool`))
  (set `self.MeshPool` _returnvalue)
  (`|ExecutionSequence`
    (:`then_0`
      (`|ExecutionSequence`
        (:`then_0`
          (bind _returnvalue_2 (`DynamicMeshPool.RequestMesh` (`self.MeshPool`)))
          (set `self.Pool Mesh 1` _returnvalue_2)
          (for _ (range (`self.Total Walls`))
            (bind (_valid_location_raw _valid_found_) (`self.Get Raw Valid Wall Position`))
            (if _valid_found_
              (bind _output_get (set `self.CurrentWallLocationRaw` _valid_location_raw))
              (`KismetArrayLibrary.Array_Add` (`self.WallLocationsRaw`) _output_get)
              (bind _cleaned_position (`self.Clean Raw Wall Position` (`self.CurrentWallLocationRaw`)))
              (set `self.CurrentWallLocationClean` _cleaned_position)
              (`GeometryScriptLibrary_MeshPrimitiveFunctions.AppendBox` (`self.Pool Mesh 1`) (struct) (`KismetMathLibrary.MakeTransform` (`KismetMathLibrary.MakeVector` _x _y) (`KismetMathLibrary.MakeRotFromXZ` (`KismetMathLibrary.MakeVector` _x _y) (0.0 0.0 1.0))) (+ (`self.LayerWidth`) (`self.WallClipTollerance`)) (`self.WallDepth`) (`self.WallHeight`) 0 0 0 "Base" null)
              (else
                (`KismetSystemLibrary.PrintString` "fffffffffffffffffffffff")))))
        (:`then_1`
          (`GeometryScriptLibrary_MeshNormalsFunctions.RecomputeNormals` (`self.Pool Mesh 1`) (struct) false null))
        (:`then_2`
          (`GeometryScriptLibrary_MeshBasicEditFunctions.AppendMesh` (`self.ViewMesh`) (`self.Pool Mesh 1`) (struct) false (struct :`CombineMode` "EnableAllMatching") null))))
    (:`then_1`
      (`self.ReleaseAllComputeMeshes`))))

(fn `Clean Raw Wall Position`
  (params (`Raw Position` :type "Vector2D Structure"))
  (returns (`Cleaned Position` :type "Vector2D Structure"))
  (locals (MyScaledPos :type "Vector2D Structure") (MySnappedPos :type "Vector2D Structure"))
  (bind _output_get (set `local.MyScaledPos` (* (- `Raw Position` (0.5 0.5)) (* (`self.TotalRadius`) 2.0))))
  (bind (_outdir _outlength) (`KismetMathLibrary.ToDirectionAndLength2D` _output_get))
  (bind _output_get_2 (set `local.MySnappedPos` (* _outdir (+ (* (`KismetMathLibrary.Round` (* (/ (- _outlength (`self.InnerRadius`)) (- (`self.TotalRadius`) (`self.InnerRadius`))) (`self.LayerCount`))) (`self.TotalLayerWidth`)) (`self.InnerRadius`) (/ (`self.LayerWidth`) 2.0) (`self.LayerSpacing`)))))
  (return _output_get_2))

(fn `Get Raw Valid Wall Position`
  (returns (`Valid Location Raw` :type "Vector2D Structure") (`Valid Found?` :type Boolean))
  (locals (MyX :type "Float (double-precision)") (MyY :type "Float (double-precision)") (`MyValid?` :type Boolean) (MyAttemptCount :type Integer) (`MyValidFound?` :type Boolean :default true))
  (bind _returnvalue (`KismetMathLibrary.RandomFloat`))
  (while (not (`local.MyValid?`))
    (`/Engine/EditorBlueprintResources/StandardMacros.IncrementInt` (`local.MyAttemptCount`)
      (:`  `
        (set `local.MyValid?` true)
        (set `local.MyX` _returnvalue)
        (set `local.MyY` _returnvalue)
        (`|ExecutionSequence`
          (:`then_0`
            (if (> (`KismetMathLibrary.DistanceSquared2D` (`KismetMathLibrary.MakeVector2D` (`local.MyX`) (`local.MyY`)) (0.5 0.5)) 0.25)
              (set `local.MyValid?` false)))
          (:`then_1`
            (if (< (`KismetMathLibrary.DistanceSquared2D` (`KismetMathLibrary.MakeVector2D` (`local.MyX`) (`local.MyY`)) (0.5 0.5)) (`KismetMathLibrary.Square` (* (/ (`self.InnerRadius`) (`self.TotalRadius`)) 0.5)))
              (set `local.MyValid?` false)))
          (:`then_2`
            (if (`self.Enforce Min Seperation?`)
              (for _array_element (`self.WallLocationsRaw`)
                (if (< (`KismetMathLibrary.DistanceSquared2D` _array_element (`KismetMathLibrary.MakeVector2D` (`local.MyX`) (`local.MyY`))) (`KismetMathLibrary.Square` (/ (`self.Min Seperation Distance`) (`self.TotalRadius`))))
                  (set `local.MyValid?` false)))))
          (:`then_3`
            (if (> (`local.MyAttemptCount`) 10)
              (set `local.MyValid?` true)
              (set `local.MyValidFound?` false)
              (`KismetSystemLibrary.PrintString` "ggggggggggggggggggggg")))))))
  (return (`KismetMathLibrary.MakeVector2D` (`local.MyX`) (`local.MyY`)) (`local.MyValidFound?`)))

(fn `UserConstructionScript`
  (set `self.TotalLayerWidth` (+ (`self.LayerWidth`) (`self.LayerSpacing`)))
  (set `self.TotalRadius` (+ (* (`self.LayerCount`) (`self.TotalLayerWidth`)) (`self.InnerRadius`))))