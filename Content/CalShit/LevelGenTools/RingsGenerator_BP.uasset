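; Procedural level-generation tool that builds concentric ring walls as a generated dynamic mesh, using Geometry Script.
; On mesh rebuild, it revolves a rectangular wall profile once per ring, stepping the radius outward from the inner radius by corridor plus wall width.
; The rings accumulate in a pooled compute mesh, which gets recomputed normals, is appended to the target mesh and is then released.
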(event `self.OnRebuildGeneratedMesh`
  (params (TargetMesh :type "DynamicMesh Object Reference"))
  (bind _wallwidth (`self.WallWidth`))
  (bind _height (`self.Height`))
  (set `self.ViewMesh` TargetMesh)
  (bind _returnvalue (`GeometryScriptLibrary_SceneUtilityFunctions.CreateDynamicMeshPool`))
  (set `self.MeshPool` _returnvalue)
  (`|ExecutionSequence`
    (:`then_0`
      (`|ExecutionSequence`
        (:`then_0`
          (bind _returnvalue_2 (`DynamicMeshPool.RequestMesh` (`self.MeshPool`)))
          (set `self.Pool Mesh 1` _returnvalue_2)
          (set `self.TotalWidth` (+ (`self.CorridorWidth`) (`self.WallWidth`)))
          (for _index (range (+ (`self.RingCount`) 1))
            (set `self.CurrentRingRadius` (+ (* _index (`self.TotalWidth`)) (`self.InnerRadius`)))
            (`GeometryScriptLibrary_MeshPrimitiveFunctions.AppendRevolvePolygon` (`self.Pool Mesh 1`) (struct) (struct) (`|MakeArray` (0.0 0.0) (`KismetMathLibrary.MakeVector2D` _wallwidth) (`KismetMathLibrary.MakeVector2D` _wallwidth _height) (`KismetMathLibrary.MakeVector2D` 0.0 _height) :!type "Vector2D Structure") (struct) (`self.CurrentRingRadius`) 128 null)))
        (:`then_1`
          (`GeometryScriptLibrary_MeshNormalsFunctions.RecomputeNormals` (`self.Pool Mesh 1`) (struct) false null))
        (:`then_2`
          (`GeometryScriptLibrary_MeshBasicEditFunctions.AppendMesh` (`self.ViewMesh`) (`self.Pool Mesh 1`) (struct) false (struct :`CombineMode` "EnableAllMatching") null))))
    (:`then_1`
      (`self.ReleaseAllComputeMeshes`))))

(fn `UserConstructionScript`)