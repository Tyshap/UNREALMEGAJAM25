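; Player character Blueprint that handles Enhanced Input movement, look, sprinting and crouching.
; Sprint adds a stamina-scaled bonus to walk speed and drains stamina using delta time cached on Tick, clamped to a nonzero floor, so speed tapers rather than cutting out.
; A looping timer regenerates stamina up to a cap, even during sprint.
; Crouch squashes the capsule's Z scale and lowers base walk speed until released.
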(event `self.ReceiveBeginPlay`
  (message `EnhancedInputSubsystemInterface.AddMappingContext` (pcsubsystem `EnhancedInputLocalPlayerSubsystem` (`GameplayStatics.GetPlayerController` 0)) "/Game/TylerShit/Movement/IAMapping.IAMapping" 0 (struct))
  (`KismetSystemLibrary.K2_SetTimerDelegate` (delegate `IncreaseStamina`) 1.0 true))

(event `self.ReceiveTick`
  (params (DeltaSeconds :type "Float (single-precision)"))
  (set `self.Delta Seconds` DeltaSeconds))

(event `EnhancedInput|/Game/TylerShit/Movement/IA_Move`
  (params (ActionValue :type "Vector2D Structure") (ElapsedSeconds :type "Float (double-precision)") (TriggeredSeconds :type "Float (double-precision)") (InputAction :type "InputAction Object Reference" :default "/Game/TylerShit/Movement/IA_Move.IA_Move"))
  (bind (_returnvalue_roll _returnvalue_pitch _returnvalue_yaw) (`KismetMathLibrary.BreakRotator` (`self.GetControlRotation`)))
  ;[1 1 1] Movement
  (:`Triggered`
    (`self.AddMovementInput` (`KismetMathLibrary.GetRightVector` (`KismetMathLibrary.MakeRotator` _returnvalue_roll 0.0 _returnvalue_yaw)) ActionValue_Y)
    (`self.AddMovementInput` (`KismetMathLibrary.GetForwardVector` (`KismetMathLibrary.MakeRotator` 0.0 0.0 _returnvalue_yaw)) ActionValue_X)))

(event `EnhancedInput|/Game/TylerShit/Movement/IA_Look`
  (params (ActionValue :type "Vector2D Structure") (ElapsedSeconds :type "Float (double-precision)") (TriggeredSeconds :type "Float (double-precision)") (InputAction :type "InputAction Object Reference" :default "/Game/TylerShit/Movement/IA_Look.IA_Look"))
  ;[1 1 1] Camera
  (:`Triggered`
    (`self.AddControllerPitchInput` ActionValue_Y)
    (`self.AddControllerYawInput` ActionValue_X)))

(event `EnhancedInput|/Game/TylerShit/Movement/IA_Sprint`
  (params (ActionValue :type Boolean) (ElapsedSeconds :type "Float (double-precision)") (TriggeredSeconds :type "Float (double-precision)") (InputAction :type "InputAction Object Reference" :default "/Game/TylerShit/Movement/IA_Sprint.IA_Sprint"))
  (bind _charactermovement (`self.CharacterMovement`))
  (bind _stamina (`self.Stamina`))
  (bind _currentwalkspeed (`self.CurrentWalkSpeed`))
  ; Sprint
  (:`Triggered`
    (if (> _stamina 0.0)
      (set `CharacterMovementComponent.MaxWalkSpeed` (+ _currentwalkspeed (* _stamina 3.0)) _charactermovement)
      (`self.ReduceStamina`)))
  (:`Completed`
    (set `CharacterMovementComponent.MaxWalkSpeed` _currentwalkspeed _charactermovement)))

(event `ReduceStamina`
  ; Sprint
  (set `self.Stamina` (- (`self.Stamina`) (* 50.0 (`self.Delta Seconds`))))
  (if (< (`self.Stamina`) 10.0)
    (set `self.Stamina` 10.0)))

(event `IncreaseStamina`
  ; Sprint
  (set `self.Stamina` (+ (`self.Stamina`) 15.0))
  (if (> (`self.Stamina`) 100.0)
    (set `self.Stamina` 100.0)))

(event `EnhancedInput|/Game/TylerShit/Movement/IA_Crouch`
  (params (ActionValue :type Boolean) (ElapsedSeconds :type "Float (double-precision)") (TriggeredSeconds :type "Float (double-precision)") (InputAction :type "InputAction Object Reference" :default "/Game/TylerShit/Movement/IA_Crouch.IA_Crouch"))
  (bind _charactermovement (`self.CharacterMovement`))
  (:`Triggered`
    (`SceneComponent.SetWorldScale3D` (`self.CapsuleComponent`) (1.0 1.0 0.6))
    (set `self.CurrentWalkSpeed` 300.0)
    (set `CharacterMovementComponent.MaxWalkSpeed` 300.0 _charactermovement))
  (:`Completed`
    (`SceneComponent.SetWorldScale3D` (`self.CapsuleComponent`) (1.0 1.0 1.0))
    (set `self.CurrentWalkSpeed` 600.0)
    (set `CharacterMovementComponent.MaxWalkSpeed` 600.0 _charactermovement)))

(fn `UserConstructionScript`)